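; BP_Player is the player actor, handling shooting, health and death.
; IA_Autofire turns its 2D input into control rotation and fires while held, and IA_Fire also starts and stops firing.
; Firing uses a looping timer at a projectiles-per-second rate to spawn BP_Fire at the spawn point.
; AffectHealth applies health deltas while alive, then destroys the player and opens MapDefeat at zero health; a RespawnPlayer call is left unwired.
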(event Custom|StartFiringProjectiles
  ;[1 1 1] Tire X projectiles par seconde
  (CallFunction|FireOneProjectile)
  (Utilities|Time|SetTimerbyFunctionName 0 "FireOneProjectile" (/ 1.0 (Variables|Default|GetProjectilePerSecond)) true))

(event Custom|StopFiringProjectiles
  ;[1 1 1] Stop le fait de tirer
  (Utilities|Time|ClearTimerbyFunctionName 0 "FireOneProjectile"))

(event Custom|FireOneProjectile
  ;[1 1 1] Faire spawn un projectile
  (Game|SpawnActorfromClass "/Game/BP/BP_Fire.BP_Fire_C" (Transformation|GetWorldTransform (Variables|Default|GetProjectileSpawnPoint)) "Undefined" "MultiplyWithRoot" 0 0))

(event Custom|UpdateIsDead
  ;[1 1 1] Vérifie si les points de vie du perso sont <= 0
  (if (<= (Variables|Default|GetHealthPoint) 0.0)
    (Variables|Default|SetIsDead true)
    (else
      (Variables|Default|SetIsDead false))))

(event Input|EnhancedActionEvents|EnhancedInputActionIA_Autofire
  (params (ActionValue :type Vector%202D%20Structure) (ElapsedSeconds :type Float%20%28double-precision%29) (TriggeredSeconds :type Float%20%28double-precision%29) (InputAction :type Input%20Action%20Object%20Reference :default "/Game/Inputs/IA_Autofire.IA_Autofire"))
  ;[1 1 1] Gère l'orientation
  ;;[1 1 1] Gère l'orientation
  (:Triggered
    (Pawn|SetControlRotation (Game|GetPlayerController 0) (Math|Conversions|RotationFromXVector (Math|Vector|MakeVector (.y ActionValue) (.x ActionValue) 0.0))))
  (:Started
    (CallFunction|StartFiringProjectiles))
  (:Completed
    (CallFunction|StopFiringProjectiles)))

(event Input|EnhancedActionEvents|EnhancedInputActionIA_Autofire
  (params (ActionValue :type Vector%202D%20Structure) (ElapsedSeconds :type Float%20%28double-precision%29) (TriggeredSeconds :type Float%20%28double-precision%29) (InputAction :type Input%20Action%20Object%20Reference :default "/Game/Inputs/IA_Autofire.IA_Autofire"))
  ;[1 1 1] Gère l'orientation
  ;;[1 1 1] Gère l'orientation
  (:Triggered
    (Pawn|SetControlRotation (Game|GetPlayerController 0) (Math|Conversions|RotationFromXVector (Math|Vector|MakeVector (.y ActionValue) (.x ActionValue) 0.0))))
  (:Started
    (CallFunction|StartFiringProjectiles))
  (:Completed
    (CallFunction|StopFiringProjectiles)))

(event Input|EnhancedActionEvents|EnhancedInputActionIA_Fire
  (params (ActionValue :type Boolean) (ElapsedSeconds :type Float%20%28double-precision%29) (TriggeredSeconds :type Float%20%28double-precision%29) (InputAction :type Input%20Action%20Object%20Reference :default "/Game/Inputs/IA_Fire.IA_Fire"))
  ;[1 1 1] Gère le tire de projectile
  (:Started
    (CallFunction|StartFiringProjectiles))
  (:Completed
    (CallFunction|StopFiringProjectiles)))

(event EventAffectHealth
  (params (Delta :type Float%20%28double-precision%29))
  ;[1 1 1] Gère la prise de dégat du player que lorsque le player n'est pas mort
  (if (not (Variables|Default|GetIsDead))
    (bind _newhealth (CallFunction|UpdateHealthPoint Delta))
    (Development|PrintString (Utilities|String|Append "PV Player = " (Utilities|String|ToString(Float) _newhealth)) true true "(R=1.000000,G=0.069327,B=0.000000,A=1.000000)")
    (if (Variables|Default|GetIsDead)
      (Actor|DestroyActor)
      (Game|OpenLevel(byName) "MapDefeat"))))

(fn ConstructionScript)

(fn UpdateHealthPoint
  (params (Delta :type Float%20%28double-precision%29))
  ;[1 1 1] Mets à jour les points de vie
  (bind _output_get (Variables|Default|SetHealthPoint (+ Delta (Variables|Default|GetHealthPoint))))
  (CallFunction|UpdateIsDead)
  (return _output_get))