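; PC_Player is the player controller that turns Enhanced Input into top-down style movement and aiming.
; BeginPlay adds IMC_Player, and IA_Move moves the player character along fixed world X and Y axes.
; IA_Autofire converts its 2D input into a control rotation for facing, without firing anything.
; Mouse-cursor aiming, noted as broken, and start/stop projectile calls are left unconnected and never run.
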(event Input|EnhancedActionEvents|EnhancedInputActionIA_Move
  (params (ActionValue :type Vector%202D%20Structure) (ElapsedSeconds :type Float%20%28double-precision%29) (TriggeredSeconds :type Float%20%28double-precision%29) (InputAction :type Input%20Action%20Object%20Reference :default "/Game/Inputs/IA_Move.IA_Move"))
  (bind _returnvalue (Game|GetPlayerCharacter 0))
  ;[1 1 1] Gère les déplacements
  (:Triggered
    (Pawn|Input|AddMovementInput _returnvalue "0.000000,1.000000,0.000000" (.x ActionValue) false) ; Horizontaux
    (Pawn|Input|AddMovementInput _returnvalue "1.000000,0.000000,0.000000" (.y ActionValue) false) ; Verticaux
  ))

(event Input|EnhancedActionEvents|EnhancedInputActionIA_Mouse
  (params (ActionValue :type Boolean) (ElapsedSeconds :type Float%20%28double-precision%29) (TriggeredSeconds :type Float%20%28double-precision%29) (InputAction :type Input%20Action%20Object%20Reference :default "/Game/Inputs/IA_Mouse.IA_Mouse"))
  ;[1 1 1] Oritentation avec la souris NE FONCTIONNE PAS
)

(event Input|EnhancedActionEvents|EnhancedInputActionIA_Autofire
  (params (ActionValue :type Vector%202D%20Structure) (ElapsedSeconds :type Float%20%28double-precision%29) (TriggeredSeconds :type Float%20%28double-precision%29) (InputAction :type Input%20Action%20Object%20Reference :default "/Game/Inputs/IA_Autofire.IA_Autofire"))
  ;[1 1 1] Gère l'orientation
  (:Triggered
    (Pawn|SetControlRotation (Game|GetPlayerController 0) (Math|Conversions|RotationFromXVector (Math|Vector|MakeVector (.y ActionValue) (.x ActionValue) 0.0)))))

(event Input|EnhancedActionEvents|EnhancedInputActionIA_Fire
  (params (ActionValue :type Boolean) (ElapsedSeconds :type Float%20%28double-precision%29) (TriggeredSeconds :type Float%20%28double-precision%29) (InputAction :type Input%20Action%20Object%20Reference :default "/Game/Inputs/IA_Fire.IA_Fire"))
  ;[1 1 1] Gère le tire de projectile
)

(event EventBeginPlay
  ;[1 1 1] Configuration des touches
  (Input|AddMappingContext (PlayerController|LocalPlayerSubsystems|GetEnhancedInputLocalPlayerSubsystem (Game|GetPlayerController 0)) "/Game/Inputs/IMC_Player.IMC_Player" 0 "(bIgnoreAllPressedKeysUntilRelease=True,bForceImmediately=False)"))

(event EventTick
  (params (DeltaSeconds :type Float%20%28single-precision%29)))

(fn ConstructionScript)