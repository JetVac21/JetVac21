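; GM_SC is the game manager that handles score, player respawn and enemy population.
; It creates the WBP_IGHUD widget and feeds it score increments, and respawns BP_Hero at the stored start transform, then possesses it.
; Registering a spawner starts a looping timer at the EnnemyPerSecond rate.
; It tracks the enemy count, exposes a check against MaxEnemyCount, and prints the count each tick.
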(event Custom|RespawnPlayer
  ;[1 1 1] Fait apparaitre une nouvelle instance et en prend le contrôle
  (bind _returnvalue (Game|SpawnActorfromClass "/Game/BP/BP_Hero.BP_Hero_C" (Variables|Default|GetPlayerSpawnTransform) "Undefined" "MultiplyWithRoot" 0 0))
  (Pawn|Possess (Game|GetPlayerController 0) _returnvalue))

(event EventBeginPlay
  ;[1 1 1] Créer le widget du score et du timer et l'affiche dans le jeu
  (bind _returnvalue (UserInterface|CreateWidget "/Game/UI/WBP_IGHUD.WBP_IGHUD_C"))
  (bind _output_get (Variables|Default|SetWidget _returnvalue))
  (UserInterface|Viewport|AddtoViewport _output_get 0))

(event EventRegisterSpawner
  (params (NewSpawner :type Bp%20Spawn%20Enemy%20Object%20Reference))
  ;[1 1 1] Enregistre le spawner placé dans le monde et lui demande de faire spawn un ennemi
  (bind _output_get (Variables|Default|SetEnnemySpawner NewSpawner))
  (Utilities|Time|SetTimerbyEvent (EventDispatchers|CreateEvent _output_get :!event SpawnOneEnemy) (/ 1.0 (Variables|Default|GetEnnemyPerSecond)) true))

(event EventIncrementEnemyCount
  ;[1 1 1] Met à jour le compteur d'ennemi sur la map
  (Math|Integer|IncrementInt (Variables|Default|GetCurentEnemyCount)))

(event EventDecrementEnemyCount
  ;[1 1 1] Met à jour le compteur d'ennemi sur la map
  (Math|Integer|DecrementInt (Variables|Default|GetCurentEnemyCount)))

(event EventTick
  (params (DeltaSeconds :type Float%20%28single-precision%29))
  ;[1 1 1] Affiche le nombre d'ennemis en jeu
  (Development|PrintString (Utilities|String|Append "NBre Ennemi = " (Utilities|String|ToString(Integer) (Variables|Default|GetCurentEnemyCount))) true true "(R=1.000000,G=0.941159,B=0.000000,A=1.000000)" 0.0))

(event EventUpdateUIScore
  ;[1 1 1] Mets à jour le score et l'envoi au widget
  (bind _result (Math|Integer|IncrementInt (Variables|Default|GetCurentScore))
    (:%20%20
      (Default|UpdateScore (Variables|Default|GetWidget) _result))))

(fn ConstructionScript)

(fn SetPlayerSpawnTransform
  (params (PlayerSpawnTransform :type Transform))
  ;[1 1 1] Stock la position de départ du joueur
  (Variables|Default|SetPlayerSpawnTransform PlayerSpawnTransform)
  (return))

(fn CanSpawnOneEnemy
  ;[1 1 1] Spawn d'ennemi si le nombre max n'est pas atteint
  (return (< (Variables|Default|GetCurentEnemyCount) (Variables|Default|GetMaxEnemyCount))))

(fn GetEnemyCount
  ;[1 1 1] Récupère le nombre d'ennemi sur la map
  (return (Variables|Default|GetCurentEnemyCount)))